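; Basic game mode that switches the player between full control, restricted cinematic control and full cinematic control, based on game and plot context.
; OnGameContextUpdate routes both Alive contexts to PlotControl, which toggles input or movement mode and jump velocity.
; Full cinematic control disables input and runs a timeline that yaws the view toward a focal location.
; BeginPlay runs a timed switch into cinematic control, then back to player control.
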(event `self.ReceiveBeginPlay`
  (`KismetSystemLibrary.Delay` 5.0)
  (`self.OnGameContextUpdate` "NewEnumerator3" "NewEnumerator2" true)
  (`KismetSystemLibrary.Delay` 3.0)
  (`self.OnGameContextUpdate` "NewEnumerator3" "NewEnumerator0" true))

(event `OrientPlayerToCinematicFocalPoint`
  (bind _returnvalue (`GameplayStatics.GetPlayerCharacter` 0))
  (bind (_initrotation_roll _initrotation_pitch _initrotation_yaw) (`KismetMathLibrary.BreakRotator` (`self.InitRotation`)))
  (bind (_targetrotation_roll _targetrotation_pitch _targetrotation_yaw) (`KismetMathLibrary.BreakRotator` (`self.TargetRotation`)))
  (bind _output_get (set `self.InitRotation` (`Controller.GetControlRotation` (`GameplayStatics.GetPlayerController` 0))))
  (set `self.TargetRotation` (`KismetMathLibrary.ComposeRotators` _output_get (`KismetMathLibrary.InverseTransformRotation` (`self.GetTransform` _returnvalue) (`KismetMathLibrary.FindLookAtRotation` (`self.K2_GetActorLocation` _returnvalue) (`self.loc`)))))
  (bind (_direction _rotationlerpalpha) (`Timeline|OrientPlayerRotation_Lerp` :!via `PlayFromStart`)
    (:`Update`
      (`Controller.SetControlRotation` (`GameplayStatics.GetPlayerController` 0) (`KismetMathLibrary.RLerp` (`KismetMathLibrary.MakeRotator` _initrotation_roll _initrotation_pitch _initrotation_yaw) (`KismetMathLibrary.MakeRotator` _initrotation_roll _initrotation_pitch _targetrotation_yaw) _rotationlerpalpha true)))))

(fn `OnGameContextUpdate`
  (params (GameControlContext :type "/Game/GameFramework/GameContext_Enum Enum" :default "NewEnumerator0") (PlotContext :type "/Game/GameFramework/PlotControlContext_Enum Enum" :default "NewEnumerator0") (PlotModifiedToo :type Boolean))
  (bind _output_get (set `self.GameContext` GameControlContext))
  (switch `/Game/GameFramework/GameContext_Enum` _output_get
    (:`NewEnumerator1`
      _)
    (:`NewEnumerator3`
      _))
  (`self.PlotControl` (select `bool` PlotModifiedToo :`false` (`self.PlotControlContext`) :`true` PlotContext)))

(fn `PlotControl`
  (params (PlotContext :type "/Game/GameFramework/PlotControlContext_Enum Enum" :default "NewEnumerator0"))
  (bind _output_get (set `self.PlotControlContext` PlotContext))
  (switch `/Game/GameFramework/PlotControlContext_Enum` _output_get
    (:`NewEnumerator0`
      (`self.SetPlotEntityControlled`))
    (:`NewEnumerator1`
      (`self.SetPlotEntityCinematicControlled`))
    (:`NewEnumerator2`
      (`self.SetPlotCinematicControlled`))))

(fn `SetPlotCinematicControlled`
  (`self.DisableInput` (`GameplayStatics.GetPlayerCharacter` 0) (`GameplayStatics.GetPlayerController` 0))
  (`self.OrientPlayerToCinematicFocalPoint`))

(fn `SetPlotEntityCinematicControlled`
  (bind _charactermovement (`Character.CharacterMovement` (`GameplayStatics.GetPlayerCharacter` 0)))
  (`CharacterMovementComponent.SetMovementMode` _charactermovement "MOVE_None" 0)
  (set `self.PreviousJumpZVelocity` (`CharacterMovementComponent.JumpZVelocity` _charactermovement))
  (set `CharacterMovementComponent.JumpZVelocity` 0.0 _charactermovement))

(fn `SetPlotEntityControlled`
  (bind _charactermovement (`Character.CharacterMovement` (`GameplayStatics.GetPlayerCharacter` 0)))
  (`self.EnableInput` (`GameplayStatics.GetPlayerCharacter` 0) (`GameplayStatics.GetPlayerController` 0))
  (`CharacterMovementComponent.SetMovementMode` _charactermovement "MOVE_Walking" 0)
  (set `CharacterMovementComponent.JumpZVelocity` (`self.PreviousJumpZVelocity`) _charactermovement))

(fn `UserConstructionScript`)