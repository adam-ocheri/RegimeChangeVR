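; Base projectile for enemy bot and player shots, launched at a random speed between its force limits, with a muzzle flash on spawn.
; A Player flag sets whether its sphere blocks Pawn or PhysicsBody, and a 10-second timer destroys it.
; Hitting an EntityBase applies damage to the player or living entities, recording bone and scaled impulse for non-players.
; Impact effects and destruction on hit follow the EntityBase cast.
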(event `self.ReceiveBeginPlay`
  (bind _sphere (`self.Sphere`))
  (`NiagaraFunctionLibrary.SpawnSystemAtLocation` "/Game/NiagaraParticleSystems/MuzzleFlashBase_NS.MuzzleFlashBase_NS" (`self.K2_GetActorLocation`) (`self.K2_GetActorRotation`))
  (bind _returnvalue (`KismetSystemLibrary.K2_SetTimerDelegate` (delegate `OnBecameIrrelevant`) 10.0))
  (set `self.BecameIrrelevant_TimerHandle` _returnvalue)
  (if (`self.Player`)
    (`PrimitiveComponent.SetCollisionResponseToChannel` _sphere "ECC_Pawn" "ECR_Ignore")
    (`PrimitiveComponent.SetCollisionResponseToChannel` _sphere "ECC_PhysicsBody" "ECR_Block")
    (else
      (`PrimitiveComponent.SetCollisionResponseToChannel` _sphere "ECC_Pawn" "ECR_Block")
      (`PrimitiveComponent.SetCollisionResponseToChannel` _sphere "ECC_PhysicsBody" "ECR_Ignore"))))

(event `OnBecameIrrelevant`
  (`self.K2_DestroyActor`))

(event `self.Sphere.OnComponentHit`
  (params (HitComponent :type "PrimitiveComponent Object Reference") (OtherActor :type "Actor Object Reference") (OtherComp :type "PrimitiveComponent Object Reference") (NormalImpulse :type "Vector Structure") (Hit :type "HitResult Structure (by ref)"))
  (bind (_bblockinghit _binitialoverlap _time _distance _location _impactpoint _normal _impactnormal _physmat _hitactor _hitcomponent _hitbonename) (`GameplayStatics.BreakHitResult` Hit))
  (bind _asentity_base (cast `EntityBase` OtherActor))
  (if (!= _asentity_base (`GameplayStatics.GetPlayerCharacter` 0))
    (if (`HealthComponent.GetIsAlive` (`EntityBase.HealthComponent` _asentity_base))
      (`EntityBase.AddHitBone` _asentity_base _hitbonename (* NormalImpulse 1e-06))
      (`GameplayStatics.ApplyDamage` null 1.0 null (`self.GetOwner`) :!label _label))
    (else
      (goto _label)))
  (`NiagaraFunctionLibrary.SpawnSystemAtLocation` "/Game/NiagaraParticleSystems/DirectionalImpact_NS.DirectionalImpact_NS" _location (`KismetMathLibrary.MakeRotFromX` _impactnormal))
  (`self.K2_DestroyActor`))

(fn `UserConstructionScript`
  (locals (InitForce :type "Float (double-precision)" :default 0.0))
  (bind _projectilemovement (`self.ProjectileMovement`))
  (bind _output_get (set `local.InitForce` (`KismetMathLibrary.RandomFloatInRange` (`self.ForceMin`) (`self.ForceMax`))))
  (set `ProjectileMovementComponent.InitialSpeed` _output_get _projectilemovement)
  (set `ProjectileMovementComponent.MaxSpeed` _output_get _projectilemovement)
  (set `MovementComponent.Velocity` (`KismetMathLibrary.MakeVector` _output_get) _projectilemovement))