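; Enemy bot character with health, a faction ID and projectile attacks fired from its left or right arm socket.
; HealthComponent events update an overhead health widget, shown for a few seconds after each change via a restarted timer.
; On death it announces the event, disables capsule collision and hides the widget.
; State updates switch walk speed between slow patrol and fast attack, while query functions expose faction and alive status.
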(event `self.ReceiveBeginPlay`
  (bind _asgeneral_entity_health_wbp (cast `/Game/Widgets/GeneralEntityHealth_WBP` (`WidgetComponent.GetWidget` (`self.Widget`))))
  (`/Game/Widgets/GeneralEntityHealth_WBP.UpdateHealth` _asgeneral_entity_health_wbp (`HealthComponent.Health` (`self.HealthComponent`))))

(event `DamagedDelegate` :!signature `self.OnTakeAnyDamage`
  (params (DamagedActor :type "Actor Object Reference") (Damage :type "Float (single-precision)") (DamageType :type "DamageType Object Reference") (InstigatedBy :type "Controller Object Reference") (DamageCauser :type "Actor Object Reference")))

(event `self.HealthComponent.EventOnDied`
  (`self.OnEntityDied`)
  (`PrimitiveComponent.SetCollisionEnabled` (`self.CapsuleComponent`) "NoCollision")
  (`self.TurnOffWidget`))

(event `self.HealthComponent.EventHealthChanged`
  (params (NewHealth :type "Float (single-precision)"))
  (`KismetSystemLibrary.K2_ClearAndInvalidateTimerHandle` (`self.HealthUpdate_TimerHandle`))
  (bind _asgeneral_entity_health_wbp (cast `/Game/Widgets/GeneralEntityHealth_WBP` (`WidgetComponent.GetWidget` (`self.Widget`))))
  (`/Game/Widgets/GeneralEntityHealth_WBP.UpdateHealth` _asgeneral_entity_health_wbp NewHealth)
  (`SceneComponent.SetVisibility` (`self.Widget`) true false)
  (bind _returnvalue (`KismetSystemLibrary.K2_SetTimerDelegate` (delegate `TurnOffWidget`) 5.0))
  (set `self.HealthUpdate_TimerHandle` _returnvalue))

(event `TurnOffWidget`
  (`SceneComponent.SetVisibility` (`self.Widget`) false false))

(fn `AttackEnemy`
  (params (EnemyTarget :type "Actor Object Reference") (Left :type Boolean))
  (`|SpawnActorFromClass` "/Game/Enemies/EnemyBot/ProjectileBase_BP.ProjectileBase_BP_C" (`SceneComponent.GetSocketTransform` (`self.Mesh`) (select `bool` Left :`false` "DEF_Arm_R_002" :`true` "DEF_Arm_L_002" :!type "Name") "RTS_World") "Undefined" "MultiplyWithRoot" self false null))

(fn `GetFactionID`
  (returns (FactionID :type String))
  (return (`self.Faction ID`)))

(fn `IsAlive`
  (returns (IsAlive :type Boolean))
  (return (`HealthComponent.GetIsAlive` (`self.HealthComponent`))))

(fn `OnStateUpdated`
  (params (NewState :type "/Game/Enemies/AIStateBase_Enum Enum" :default "NewEnumerator0"))
  (bind _charactermovement (`self.CharacterMovement`))
  (switch `/Game/Enemies/AIStateBase_Enum` NewState
    (:`NewEnumerator1`
      (set `CharacterMovementComponent.MaxWalkSpeed` 150.0 _charactermovement))
    (:`NewEnumerator2`
      (set `CharacterMovementComponent.MaxWalkSpeed` 600.0 _charactermovement))))

(fn `UserConstructionScript`)