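; EntityBase_BP is an enemy base Blueprint that gives physical hit reactions on its skeletal mesh.
; OnDamageImpact records the struck bone in the BoneHitData map, turns on physics simulation and full blend weight for that bone and those below, then applies a scaled impulse.
; Tick scans the map for positive values but does nothing with them, so no blend-back to animation happens here.
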(event `self.ReceiveTick`
  (params (DeltaSeconds :type "Float (single-precision)"))
  (bind _bonehitdata (`self.BoneHitData`))
  (bind _keys (`BlueprintMapLibrary.Map_Keys` _bonehitdata))
  (for _array_element _keys
    (bind (_value _returnvalue) (`BlueprintMapLibrary.Map_Find` _bonehitdata _array_element))
    (if _returnvalue
      (if (> _value 0.0)
        _))))

(fn `OnDamageImpact`
  (params (InBoneName :type "Name (by ref)") (A :type "Vector Structure"))
  (bind _mesh (`self.Mesh`))
  (`BlueprintMapLibrary.Map_Add` (`self.BoneHitData`) InBoneName 1.0)
  (`SkeletalMeshComponent.SetAllBodiesBelowSimulatePhysics` _mesh InBoneName true true)
  (`SkeletalMeshComponent.SetAllBodiesBelowPhysicsBlendWeight` _mesh InBoneName 1.0 false true)
  (`SkeletalMeshComponent.AddImpulseToAllBodiesBelow` _mesh (* A 1000.0) InBoneName false true))

(fn `UserConstructionScript`)