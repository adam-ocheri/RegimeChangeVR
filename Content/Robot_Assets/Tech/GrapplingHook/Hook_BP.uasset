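; Grappling hook projectile that launches along its forward vector and stops where it first hits.
; On BeginPlay a velocity-change impulse sends the physics collider forward, using a force the construction script takes from a default-built rank parameters struct.
; On hit it disables gravity, physics simulation and collision to freeze in place, then sets the HookLatchedOn flag.
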(event `self.ReceiveBeginPlay`
  (`self.ApplyInitialForces` (`self.InitForce`)))

(event `self.Collider.OnComponentHit`
  (params (HitComponent :type "PrimitiveComponent Object Reference") (OtherActor :type "Actor Object Reference") (OtherComp :type "PrimitiveComponent Object Reference") (NormalImpulse :type "Vector Structure") (Hit :type "HitResult Structure (by ref)"))
  (`self.CeaseMovement`)
  (`self.OnHookLatchedOn`))

(fn `ApplyInitialForces`
  (params (InitForceMultiplier :type "Float (double-precision)"))
  (`PrimitiveComponent.AddImpulse` (`self.Collider`) (* (`self.GetActorForwardVector`) InitForceMultiplier) "None" true))

(fn `CeaseMovement`
  (bind _collider (`self.Collider`))
  (`PrimitiveComponent.SetEnableGravity` _collider false)
  (`PrimitiveComponent.SetSimulatePhysics` _collider false)
  (`PrimitiveComponent.SetCollisionEnabled` _collider "NoCollision"))

(fn `OnHookLatchedOn`
  (set `self.HookLatchedOn` true))

(fn `UserConstructionScript`
  (set `self.InitForce` (`.HookInitForce_10_FEC6D846488F5E8CFC09238C36C1C031` (break `/Game/Robot_Assets/RankParameters_UStruct` (make `/Game/Robot_Assets/RankParameters_UStruct` false)))))