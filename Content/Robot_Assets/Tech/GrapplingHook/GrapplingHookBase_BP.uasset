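; Base actor for the VR robot's grappling hook, linking a cable to a separately spawned hook actor.
; On BeginPlay it spawns the hook at the right-arm socket of the player robot's mesh and attaches the cable end to the hook's collider.
; OnHookReleased clears the hook's latched state and stops its movement.
; Destroying the base also destroys the hook.
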(event `self.ReceiveBeginPlay`
  (bind _asvrbot_char_bp (cast `/Game/Robot_Assets/VRBot_Char_BP` (`GameplayStatics.GetPlayerCharacter` 0)))
  (bind _returnvalue (`|SpawnActorFromClass` "/Game/Robot_Assets/Tech/GrapplingHook/Hook_BP.Hook_BP_C" (`SceneComponent.GetSocketTransform` (`Character.Mesh` _asvrbot_char_bp) "DEF_Arm_R_003" "RTS_World") "Undefined" "MultiplyWithRoot" null null))
  (bind _output_get (set `self.Hook_BP` _returnvalue))
  (`CableComponent.SetAttachEndTo` (`self.Cable`) _output_get "Collider" "None"))

(event `self.ReceiveDestroyed`
  (`self.K2_DestroyActor` (`self.Hook_BP`)))

(fn `OnHookReleased`
  (bind _hook_bp (`self.Hook_BP`))
  (set `/Game/Robot_Assets/Tech/GrapplingHook/Hook_BP.HookLatchedOn` false _hook_bp)
  (`/Game/Robot_Assets/Tech/GrapplingHook/Hook_BP.CeaseMovement` _hook_bp))

(fn `UserConstructionScript`)