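; Robot audio actor that drives movement sounds from head, hand and locomotion velocities.
; On BeginPlay it spawns and attaches a VelocityTracker_BP, whose socket names place the center, left and right audio components on a skeletal mesh, with root audio at the pelvis.
; CoreUpdate, rather than its empty Tick, updates the tracker, then feeds velocities into each component's float parameters for head, arms, walk and turn.
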(event `self.ReceiveBeginPlay`
  (bind _returnvalue (`|SpawnActorFromClass` "/Game/Robot_Assets/Audio/VelocityTracker_BP.VelocityTracker_BP_C" (`self.GetTransform`) "Undefined" "MultiplyWithRoot" null null))
  (bind _output_get (set `self.VelocityTracker` _returnvalue))
  (`self.K2_AttachToActor` _output_get self "None" "SnapToTarget" "SnapToTarget" "KeepWorld" true))

(event `self.ReceiveTick`
  (params (DeltaSeconds :type "Float (single-precision)")))

(fn `ApplyVelocityToAudio`
  (params (VelocityTracker :type "/Game/Robot_Assets/Audio/VelocityTracker_BP Object Reference"))
  (bind (_headvelocity _leftvelocity _rightvelocity) (`/Game/Robot_Assets/Audio/VelocityTracker_BP.GetSocketsVelocity` VelocityTracker))
  (bind (_up _right _turn) (`/Game/Robot_Assets/Audio/VelocityTracker_BP.GetInputAxesVelocity` VelocityTracker))
  (bind _audio_root (`self.Audio_Root`))
  (`AudioParameterControllerInterface.SetFloatParameter` (`self.Audio_Center`) "Head" _headvelocity)
  (`AudioParameterControllerInterface.SetFloatParameter` (`self.Audio_Left`) "LeftArm" _leftvelocity)
  (`AudioParameterControllerInterface.SetFloatParameter` (`self.Audio_Right`) "RightArm" _rightvelocity)
  (`AudioParameterControllerInterface.SetFloatParameter` _audio_root "Walk" (/ (+ _up _right) 2.0))
  (`AudioParameterControllerInterface.SetFloatParameter` _audio_root "Turn" _turn))

(fn `AttachSoundSourcesToBones`
  (params (TargetSkeletalMesh :type "SkeletalMeshComponent Object Reference"))
  (bind (_headsocketname _lefthandsocketname _righthandsocketname) (`/Game/Robot_Assets/Audio/VelocityTracker_BP.GetSocketNames` (`self.VelocityTracker`)))
  (`SceneComponent.K2_AttachToComponent` (`self.Audio_Center`) TargetSkeletalMesh _headsocketname "KeepWorld" "KeepWorld" "KeepWorld" true)
  (`SceneComponent.K2_AttachToComponent` (`self.Audio_Left`) TargetSkeletalMesh _lefthandsocketname "SnapToTarget" "SnapToTarget" "KeepWorld" true)
  (`SceneComponent.K2_AttachToComponent` (`self.Audio_Right`) TargetSkeletalMesh _righthandsocketname "SnapToTarget" "SnapToTarget" "KeepWorld" true)
  (`SceneComponent.K2_AttachToComponent` (`self.Audio_Root`) TargetSkeletalMesh "DEF_PelvisBase_001" "SnapToTarget" "SnapToTarget" "KeepWorld" true))

(fn `CoreUpdate`
  (params (`SK Mesh Comp` :type "SkeletalMeshComponent Object Reference") (DeltaSeconds :type "Float (double-precision)"))
  (bind _velocitytracker (`self.VelocityTracker`))
  (`/Game/Robot_Assets/Audio/VelocityTracker_BP.CoreVelocityUpdate` _velocitytracker `SK Mesh Comp` DeltaSeconds)
  (`self.ApplyVelocityToAudio` _velocitytracker))

(fn `UserConstructionScript`)