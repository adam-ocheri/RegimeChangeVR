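; Velocity tracker Blueprint in the robot audio assets that measures motion of the head, both arms and the walk and turn input axes.
; CoreVelocityUpdate is driven externally rather than by Tick, feeding a skeletal mesh and delta time to bone and parameter velocity components.
; Bone components alternate up-frame and down-frame calculations on successive calls, while axis components update every call.
; Getters expose the resulting velocities and tracked socket names.
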(event `self.ReceiveBeginPlay`)

(event `self.ReceiveTick`
  (params (DeltaSeconds :type "Float (single-precision)")))

(fn `CoreVelocityUpdate`
  (params (`SK Mesh Comp` :type "SkeletalMeshComponent Object Reference") (DeltaSeconds :type "Float (double-precision)"))
  (bind _bonevelocitycomponent_leftarm (`self.BoneVelocityComponent_LeftArm`))
  (`/Engine/EditorBlueprintResources/StandardMacros.IsValid` `SK Mesh Comp`
    (:`Is Valid`
      (if (`self.UpFrame`)
        (`/Game/Robot_Assets/BoneVelocityComponent.CalculateUpFrame` _bonevelocitycomponent_leftarm `SK Mesh Comp` DeltaSeconds)
        (`/Game/Robot_Assets/BoneVelocityComponent.CalculateUpFrame` (`self.BoneVelocityComponent_RightArm`) `SK Mesh Comp` DeltaSeconds)
        (`/Game/Robot_Assets/BoneVelocityComponent.CalculateUpFrame` (`self.BoneVelocityComponent_Head`) `SK Mesh Comp` DeltaSeconds)
        (set `self.UpFrame` false)
        (else
          (`/Game/Robot_Assets/BoneVelocityComponent.CalculateDownFrame` _bonevelocitycomponent_leftarm `SK Mesh Comp` DeltaSeconds)
          (`/Game/Robot_Assets/BoneVelocityComponent.CalculateDownFrame` (`self.BoneVelocityComponent_RightArm`) `SK Mesh Comp` DeltaSeconds)
          (`/Game/Robot_Assets/BoneVelocityComponent.CalculateDownFrame` (`self.BoneVelocityComponent_Head`) `SK Mesh Comp` DeltaSeconds)
          (set `self.UpFrame` true)))
      (`/Game/Robot_Assets/ParameterVelocityComponent.UpdateVelocity` (`self.ParameterVelocityComponent_Walk_XAxis`) DeltaSeconds)
      (`/Game/Robot_Assets/ParameterVelocityComponent.UpdateVelocity` (`self.ParameterVelocityComponent_Walk_YAxis`) DeltaSeconds)
      (`/Game/Robot_Assets/ParameterVelocityComponent.UpdateVelocity` (`self.ParameterVelocityComponent_Turn_XAxis`) DeltaSeconds))))

(fn `GetInputAxesVelocity`
  (returns (Up :type "Float (double-precision)") (Right :type "Float (double-precision)") (Turn :type "Float (double-precision)"))
  (return (`/Game/Robot_Assets/ParameterVelocityComponent.GetUpdatedVelocity` (`self.ParameterVelocityComponent_Walk_YAxis`)) (`/Game/Robot_Assets/ParameterVelocityComponent.GetUpdatedVelocity` (`self.ParameterVelocityComponent_Turn_XAxis`)) (`/Game/Robot_Assets/ParameterVelocityComponent.GetUpdatedVelocity` (`self.ParameterVelocityComponent_Walk_XAxis`))))

(fn `GetSocketNames`
  (returns (HeadSocketName :type Name) (LeftHandSocketName :type Name) (RightHandSocketName :type Name))
  (return (`/Game/Robot_Assets/BoneVelocityComponent.SocketName` (`self.BoneVelocityComponent_Head`)) (`/Game/Robot_Assets/BoneVelocityComponent.SocketName` (`self.BoneVelocityComponent_LeftArm`)) (`/Game/Robot_Assets/BoneVelocityComponent.SocketName` (`self.BoneVelocityComponent_RightArm`))))

(fn `GetSocketsVelocity`
  (returns (HeadVelocity :type "Float (double-precision)") (LeftVelocity :type "Float (double-precision)") (RightVelocity :type "Float (double-precision)"))
  (return (`/Game/Robot_Assets/BoneVelocityComponent.GetUpdatedVelocity` (`self.BoneVelocityComponent_Head`)) (`/Game/Robot_Assets/BoneVelocityComponent.GetUpdatedVelocity` (`self.BoneVelocityComponent_LeftArm`)) (`/Game/Robot_Assets/BoneVelocityComponent.GetUpdatedVelocity` (`self.BoneVelocityComponent_RightArm`))))

(fn `UserConstructionScript`)